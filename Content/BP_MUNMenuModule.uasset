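; Menu module for a mod update notifier (MUN) that collects mod info and passes update results to a menu widget.
; On Construction it spawns the MIA_MUN actor, and on Post Initialization it gathers MUNInfo from every MUNInfoActor and calls Init with the list.
; Info actors in the world serve as the registration mechanism.
; When update processing finishes, it logs ModUpdates and hands it to MenuWidget.
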(event `self.FinishedProcessingUpdates`
  (bind _modupdates (`self.ModUpdates`))
  (`BlueprintLoggingLibrary.LogDisplay` (`KismetStringLibrary.Concat_StrStr` "Output list: \\n" _modupdates))
  (message `/ModUpdateNotifier/Interface/BPI_MUN.GetModUpdates` (`self.MenuWidget`) _modupdates))

(event `self.K2_OnLifecycleEvent`
  (params (Phase :type "ELifecyclePhase Enum" :default "CONSTRUCTION"))
  (bind _mod_info_list (`self.Mod Info List`))
  (switch `ELifecyclePhase` Phase
    (:`CONSTRUCTION`
      (`|SpawnActorFromClass` "/ModUpdateNotifier/MIA_MUN.MIA_MUN_C" (`KismetMathLibrary.MakeTransform` (0.0 0.0 0.0)) "Undefined" "MultiplyWithRoot" null null))
    (:`POST_INITIALIZATION`
      (bind _outactors (`GameplayStatics.GetAllActorsOfClass` "/Script/ModUpdateNotifier.MUNInfoActor"))
      (for _array_element _outactors
        (`KismetArrayLibrary.Array_Add` _mod_info_list (`MUNInfoActor.MUNInfo` _array_element)))
      (`self.Init` _mod_info_list))))